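; BP_HeartToyHolder is a collectible item holder that spawns a BP_SodaSpawn actor when the Grab input is pressed.
; Its Box overlap enables player 0's input on the holder when a Raccoon enters and disables it when the Raccoon leaves.
; Grab requires the game mode to be BP_GameModeRaccoon, then waits a short delay before spawning at a hardcoded location.
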(event OnComponentBeginOverlap(Box)
  (params (OverlappedComponent :type Primitive%20Component%20Object%20Reference) (OtherActor :type Actor%20Object%20Reference) (OtherComp :type Primitive%20Component%20Object%20Reference) (OtherBodyIndex :type Integer) (bFromSweep :type Boolean) (SweepResult :type Hit%20Result%20Structure%20%28by%20ref%29))
  (Utilities|Casting|CastToRaccoon OtherActor)
  (Input|EnableInput (Game|GetPlayerController 0)))

(event OnComponentEndOverlap(Box)
  (params (OverlappedComponent :type Primitive%20Component%20Object%20Reference) (OtherActor :type Actor%20Object%20Reference) (OtherComp :type Primitive%20Component%20Object%20Reference) (OtherBodyIndex :type Integer))
  (Utilities|Casting|CastToRaccoon OtherActor)
  (Input|DisableInput (Game|GetPlayerController 0)))

(event Input|ActionEvents|InputActionGrab
  (params (Key :type Key%20Structure :default "None"))
  (:Pressed
    (Utilities|Casting|CastToBP_GameModeRaccoon (Game|GetGameMode))
    (Utilities|FlowControl|Delay 1.0)
    (Game|SpawnActorfromClass "/Game/Blueprints/Collectibles/ItemHolders/ItemsActor/BP_SodaSpawn.BP_SodaSpawn_C" (Math|Transform|MakeTransform "261.905334,-539.032898,186.269562" "0, 0, 0" "1,1,1") "Undefined" 0 0)))

(fn ConstructionScript)