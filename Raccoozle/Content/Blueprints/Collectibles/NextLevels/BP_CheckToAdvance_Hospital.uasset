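; Level exit trigger that loads the Alley level once the raccoon game mode's ObjectsForAlley counter is zero.
; BeginPlay hides the actor only if that counter is already zero, and Tick unhides it whenever the counter reads zero.
; The collision box enables player input on the actor while the Raccoon overlaps, so pressing Grab there re-checks the counter and opens the level.
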(event OnComponentBeginOverlap(CollisionBox)
  (params (OverlappedComponent :type Primitive%20Component%20Object%20Reference) (OtherActor :type Actor%20Object%20Reference) (OtherComp :type Primitive%20Component%20Object%20Reference) (OtherBodyIndex :type Integer) (bFromSweep :type Boolean) (SweepResult :type Hit%20Result%20Structure%20%28by%20ref%29))
  (Utilities|Casting|CastToRaccoon OtherActor)
  (Input|EnableInput (Game|GetPlayerController 0)))

(event OnComponentEndOverlap(CollisionBox)
  (params (OverlappedComponent :type Primitive%20Component%20Object%20Reference) (OtherActor :type Actor%20Object%20Reference) (OtherComp :type Primitive%20Component%20Object%20Reference) (OtherBodyIndex :type Integer))
  (Utilities|Casting|CastToRaccoon OtherActor)
  (Input|DisableInput (Game|GetPlayerController 0)))

(event EventTick
  (params (DeltaSeconds :type Float%20%28single-precision%29))
  (bind _asbp_game_mode_raccoon (Utilities|Casting|CastToBP_GameModeRaccoon (Game|GetGameMode)))
  (if (== (Variables|/Game/Blueprints/BP_GameModeRaccoon.BP_GameModeRaccoon_C|GetObjects%20for%20Alley _asbp_game_mode_raccoon) 0)
    (Rendering|SetActorHiddenInGame false)))

(event EventBeginPlay
  (bind _asbp_game_mode_raccoon (Utilities|Casting|CastToBP_GameModeRaccoon (Game|GetGameMode)))
  (if (== (Variables|/Game/Blueprints/BP_GameModeRaccoon.BP_GameModeRaccoon_C|GetObjects%20for%20Alley _asbp_game_mode_raccoon) 0)
    (Rendering|SetActorHiddenInGame true)))

(event Input|ActionEvents|InputActionGrab
  (params (Key :type Key%20Structure :default "None"))
  (:Pressed
    (bind _asbp_game_mode_raccoon (Utilities|Casting|CastToBP_GameModeRaccoon (Game|GetGameMode)))
    (if (== (Variables|/Game/Blueprints/BP_GameModeRaccoon.BP_GameModeRaccoon_C|GetObjects%20for%20Alley _asbp_game_mode_raccoon) 0)
      (Game|OpenLevel(byName) "Alley"))))

(fn ConstructionScript)