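; BP_DoctorHeartTool is a collectible that the Raccoon grabs, counting down the objects tracked for the trash place.
; Its box collider enables input from player 0 while a Raccoon overlaps it and disables it when the overlap ends.
; Grab decrements ObjectsForTrashPlace on BP_GameModeRaccoon, then destroys the actor after a short delay.
; Nothing blocks repeat presses during that delay, so each one decrements the counter again.
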(event OnComponentBeginOverlap(BoxCollider)
  (params (OverlappedComponent :type Primitive%20Component%20Object%20Reference) (OtherActor :type Actor%20Object%20Reference) (OtherComp :type Primitive%20Component%20Object%20Reference) (OtherBodyIndex :type Integer) (bFromSweep :type Boolean) (SweepResult :type Hit%20Result%20Structure%20%28by%20ref%29))
  (Utilities|Casting|CastToRaccoon OtherActor)
  (Input|EnableInput (Game|GetPlayerController 0)))

(event OnComponentEndOverlap(BoxCollider)
  (params (OverlappedComponent :type Primitive%20Component%20Object%20Reference) (OtherActor :type Actor%20Object%20Reference) (OtherComp :type Primitive%20Component%20Object%20Reference) (OtherBodyIndex :type Integer))
  (Utilities|Casting|CastToRaccoon OtherActor)
  (Input|DisableInput (Game|GetPlayerController 0)))

(event Input|ActionEvents|InputActionGrab
  (params (Key :type Key%20Structure :default "None"))
  (:Pressed
    (bind _asbp_game_mode_raccoon (Utilities|Casting|CastToBP_GameModeRaccoon (Game|GetGameMode)))
    (bind _result (Math|Integer|DecrementInt (Variables|/Game/Blueprints/BP_GameModeRaccoon.BP_GameModeRaccoon_C|GetObjects%20for%20TrashPlace _asbp_game_mode_raccoon))
      (:%20%20
        (Variables|/Game/Blueprints/BP_GameModeRaccoon.BP_GameModeRaccoon_C|SetObjects%20for%20TrashPlace _asbp_game_mode_raccoon _result)
        (Utilities|FlowControl|Delay 1.0)
        (Actor|DestroyActor)))))

(fn ConstructionScript)