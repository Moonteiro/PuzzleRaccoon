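; BP_GameModeRaccoon is a game mode that tallies placed item actors for five named areas: Alley, Street, School, Hospital and TrashPlace.
; On BeginPlay, a sequence finds all soda, apple, coffee packet, book and doctor heart tool actors.
; Each count is stored in the matching area's ObjectsFor variable, in that respective order, so books count toward Hospital and coffee packets toward School.
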(event EventBeginPlay
  (Utilities|FlowControl|Sequence
    (:then_0
      (bind _outactors (Actor|GetAllActorsOfClass "/Game/Blueprints/Collectibles/BP_Soda.BP_Soda_C"))
      (Variables|Default|SetObjects%20for%20Alley (Utilities|Array|Length _outactors)))
    (:then_1
      (bind _outactors_2 (Actor|GetAllActorsOfClass "/Game/Blueprints/Collectibles/BP_Apple.BP_Apple_C"))
      (Variables|Default|SetObjects%20for%20Street (Utilities|Array|Length _outactors_2)))
    (:then_2
      (bind _outactors_3 (Actor|GetAllActorsOfClass "/Game/Blueprints/Collectibles/BP_CoffePacket.BP_CoffePacket_C"))
      (Variables|Default|SetObjects%20for%20School (Utilities|Array|Length _outactors_3)))
    (:then_3
      (bind _outactors_4 (Actor|GetAllActorsOfClass "/Game/Blueprints/Collectibles/BP_Book.BP_Book_C"))
      (Variables|Default|SetObjects%20for%20Hospital (Utilities|Array|Length _outactors_4)))
    (:then_4
      (bind _outactors_5 (Actor|GetAllActorsOfClass "/Game/Blueprints/Collectibles/BP_DoctorHeartTool.BP_DoctorHeartTool_C"))
      (Variables|Default|SetObjects%20for%20TrashPlace (Utilities|Array|Length _outactors_5)))))

(fn ConstructionScript)