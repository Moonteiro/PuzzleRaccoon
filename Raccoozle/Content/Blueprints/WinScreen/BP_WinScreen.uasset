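; BP_WinScreen is an actor that shows the win screen once the game mode reports that all objects are accounted for.
; Every Tick it casts the game mode to BP_GameModeRaccoon and checks whether AllObjects equals five.
; While that holds, it adds a new WB_WinScreen to the viewport each frame with no once-only guard, shows the mouse cursor and sets look and move input ignore to false.
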(event EventBeginPlay)

(event Collision|EventActorBeginOverlap
  (params (OtherActor :type Actor%20Object%20Reference)))

(event EventTick
  (params (DeltaSeconds :type Float%20%28single-precision%29))
  (bind _returnvalue (Game|GetPlayerController 0))
  (Utilities|FlowControl|Sequence
    (:then_0
      (bind _asbp_game_mode_raccoon (Utilities|Casting|CastToBP_GameModeRaccoon (Game|GetGameMode)))
      (if (== (Variables|/Game/Blueprints/BP_GameModeRaccoon.BP_GameModeRaccoon_C|GetAll%20Objects _asbp_game_mode_raccoon) 5)
        (bind _returnvalue_2 (UserInterface|CreateWidget "/Game/Blueprints/WinScreen/WB_WinScreen.WB_WinScreen_C"))
        (UserInterface|Viewport|AddtoViewport _returnvalue_2 0)
        (Variables|/Script/Engine.PlayerController|SetbShowMouseCursor _returnvalue true)
        (Input|SetIgnoreLookInput _returnvalue false)
        (Input|SetIgnoreMoveInput _returnvalue false)))))

(fn ConstructionScript)